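; Tower actor that procedurally covers a scalable tower mesh in randomized instanced tiles at construction time.
; The construction script scales the mesh, clears five tile instance components, then stacks rings of evenly spaced tiles around it, with radius following tower X scale.
; Each tile gets a random component, quarter-turn roll and scale.
; A decreasing, clamped spawn weight keeps lower rings full and progressively thins upper rings.
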(event EventBeginPlay)

(event Collision|EventActorBeginOverlap
  (params (OtherActor :type Actor%20Object%20Reference)))

(event EventTick
  (params (DeltaSeconds :type Float%20%28single-precision%29)))

(fn ConstructionScript
  (Transformation|SetRelativeScale3D (Variables|Default|GetTowerMesh) (Variables|Default|GetTowerScale))
  (CallFunction|ResetValues)
  (CallFunction|SpawnTiles))

(fn ComposeTransform
  (bind _returnvalue (Math|Random|RandomFloatinRange 11.0 12.0))
  (return (Math|Transform|MakeTransform (+ (Math|Vector|MakeVector 0.0 0.0 (Variables|Default|GetHeightLocation)) (* (Math|Vector|GetForwardVector (Math|Rotator|MakeRotator 0.0 0.0 (Variables|Default|GetVectorRotationOffset))) (* (Variables|Default|GetDistance) (.X (Math|Vector|BreakVector (Variables|Default|GetTowerScale)))))) (Math|Rotator|CombineRotators "90.000000, 0,0.000000" (Math|Rotator|MakeRotator (Utilities|Select :Index (Math|Random|RandomIntegerinRange 0 3) :Option%200 0.0 :Option%201 9e+01 :Option%202 1.8e+02 :Option%203 2.7e+02) 0.0 (Variables|Default|GetVectorRotationOffset))) (Math|Vector|MakeVector _returnvalue _returnvalue (Math|Random|RandomFloatinRange 1.0 5.0)))))

(fn RandomTileInstance
  (return (Utilities|Select :Index (Math|Random|RandomIntegerinRange 0 4) :Option%200 (Variables|Default|GetTowerTiles1) :Option%201 (Variables|Default|GetTowerTiles2) :Option%202 (Variables|Default|GetTowerTiles3) :Option%203 (Variables|Default|GetTowerTiles4) :Option%204 (Variables|Default|GetTowerTiles5))))

(fn SpawnTiles
  (for _index (range 0 20)
    (for _index_2 (range 0 119)
      (if (Math|Random|RandomBoolwithWeight (Math|Float|Clamp(Float) (Variables|Default|GetSpawnRatio)))
        (Components|InstancedStaticMesh|AddInstance (CallFunction|RandomTileInstance) (CallFunction|ComposeTransform)))
      (Variables|Default|SetVectorRotationOffset (* (Math|Conversions|ToFloat(Integer) (+ _index_2 1)) 3.0)))
    (Variables|Default|SetHeightLocation (+ (Variables|Default|GetHeightLocation) 2.5e+02))
    (Variables|Default|SetSpawnRatio (- (Variables|Default|GetSpawnRatio) 0.1))))

(fn ResetValues
  (Components|InstancedStaticMesh|ClearInstances (Variables|Default|GetTowerTiles1))
  (Variables|Default|SetHeightLocation -3.4e+03)
  (Variables|Default|SetSpawnRatio 2.0))
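; BP_WaterVolume is a construction-script-driven stylized water volume with a surface plane, underwater post process, caustics and optional planar reflections.
; XY scale and depth size the plane, post-process box and point light radius.
; Dynamic material instances receive the actor's height for underwater fog and for caustics projected as the point light's light function.
; A reflection toggle swaps lit and unlit water materials and shows or hides the planar reflection.
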(event EventBeginPlay)

(event Collision|EventActorBeginOverlap
  (params (OtherActor :type Actor%20Object%20Reference)))

(event EventTick
  (params (DeltaSeconds :type Float%20%28single-precision%29)))

(fn ConstructionScript
  (CallFunction|ControlComponentScaling)
  (CallFunction|ConfigureUnderwaterPP)
  (CallFunction|ControlCausticsViaLightFunction)
  (CallFunction|ControlReflections))

(fn ConfigureUnderwaterPP
  ;[1 1 1] Configure Underwater Post Process values
  (bind _returnvalue (Rendering|Material|CreateDynamicMaterialInstance "/Game/HWStylizedPond/Materials/MaterialInstances/MI_UnderWaterPostProcess.MI_UnderWaterPostProcess" "None" :!class /Script/Engine.KismetMaterialLibrary))
  (bind _output_get (Variables|Default|SetUnderWaterMaterial _returnvalue))
  (Variables|/Script/Engine.PostProcessComponent|SetSettings (Variables|Default|GetPostProcess) (Utilities|Struct|MakePostProcessSettings (Utilities|Struct|MakeWeightedBlendables (Utilities|Array|MakeArray (Utilities|Struct|MakeWeightedBlendable 1.0 _output_get)))))
  (Rendering|Material|SetScalarParameterValue (Variables|Default|GetUnderWaterMaterial) "WaterZLocation" (.z (Transformation|GetActorLocation)) :!class /Script/Engine.MaterialInstanceDynamic)
  (Rendering|Material|SetScalarParameterValue (Variables|Default|GetUnderWaterMaterial) "WaterFog" (Variables|Default|GetFogAmount) :!class /Script/Engine.MaterialInstanceDynamic))

(fn ControlComponentScaling
  (bind _xyscale (Variables|Default|GetXYScale))
  (bind _xyscale_2 (Variables|Default|GetXYScale))
  (bind _returnvalue (/ _xyscale_2 1e+02))
  ;[1 1 1] Control XY scale for water plane
  (Transformation|SetRelativeScale3D (Variables|Default|GetSM_WaterPlane) (Math|Vector|MakeVector _returnvalue _returnvalue 1.0))
  ;[1 1 1] Scale PP Volume while locking it to plane height for top sector
  (Variables|/Script/Engine.SpringArmComponent|SetTargetArmLength (Variables|Default|GetPPArm) (- (Variables|Default|GetDepth) 1e+01))
  (Components|Box|SetBoxExtent (Variables|Default|GetPPBox) (Math|Vector|MakeVector _xyscale _xyscale (Variables|Default|GetDepth)) true)
  ;[1 1 1] Control Light Falloff based on volume size
  (Rendering|Lighting|SetAttenuationRadius (Variables|Default|GetPointLight) (Math|Float|SelectFloat (* (Variables|Default|GetDepth) 3.0) (* (Variables|Default|GetXYScale) 1.5) (> (Variables|Default|GetDepth) (/ (Variables|Default|GetXYScale) 2.0)))))

(fn ControlCausticsViaLightFunction
  (bind _returnvalue (Rendering|Material|CreateDynamicMaterialInstance "/Game/HWStylizedPond/Materials/MaterialInstances/MI_CausticFunction.MI_CausticFunction" "None" :!class /Script/Engine.KismetMaterialLibrary))
  (bind _output_get (Variables|Default|SetCausticMaterial _returnvalue))
  (Rendering|Material|SetScalarParameterValue _output_get "WaterZLocation" (- (.z (Transformation|GetActorLocation)) 4e+02) :!class /Script/Engine.MaterialInstanceDynamic)
  (Rendering|Components|Light|SetLightFunctionMaterial (Variables|Default|GetPointLight) (Variables|Default|GetCausticMaterial)))

(fn ControlReflections
  ;[1 1 1] ControlReflections
  (Rendering|Material|SetMaterial (Variables|Default|GetSM_WaterPlane) 0 (select (Variables|Default|GetRenderReflections) "/Game/HWStylizedPond/Materials/MaterialInstances/MI_StylizedWater.MI_StylizedWater" "/Game/HWStylizedPond/Materials/MaterialInstances/MI_StylizedWater_Unlit.MI_StylizedWater_Unlit"))
  (Rendering|SetVisibility (Variables|Default|GetPlanarReflection) (Variables|Default|GetRenderReflections) false))